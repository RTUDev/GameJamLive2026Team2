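; BP_Hook is the hook in a baby-fishing minigame, deciding whether the caught BP_Baby is the player's own.
; On sphere overlap it compares the baby to MyBaby, then adds or removes a baby on PlayerRef and blends the view back to its camera.
; Either result re-enables input (on the hook for a match, the player otherwise), then destroys all "fish"-tagged babies and the hook.
; FishBaby is empty, and the timeline-driven vertical movement is disconnected.
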(event OnComponentBeginOverlap(SphereCollision)
  (params (OverlappedComponent :type Primitive%20Component%20Object%20Reference) (OtherActor :type Actor%20Object%20Reference) (OtherComp :type Primitive%20Component%20Object%20Reference) (OtherBodyIndex :type Integer) (bFromSweep :type Boolean) (SweepResult :type Hit%20Result%20Structure%20%28by%20ref%29))
  (bind _returnvalue (Game|GetPlayerController 0))
  (bind _returnvalue_2 (Game|GetPlayerController 0))
  (bind _playerref (Variables|Default|GetplayerRef))
  (bind _currentcamera (Variables|/Game/ThirdPerson/Blueprints/BP_ThirdPersonCharacter.BP_ThirdPersonCharacter_C|GetCurrentCamera _playerref))
  (bind _asbp_baby (Utilities|Casting|CastToBP_Baby OtherActor))
  (if (== _asbp_baby (Variables|Default|GetmyBaby))
    (Development|PrintString "That's my baby")
    (Math|Integer|IncrementInt (Variables|/Game/ThirdPerson/Blueprints/BP_ThirdPersonCharacter.BP_ThirdPersonCharacter_C|GetbabyNumber _playerref)
      (:%20%20
        (Game|Player|SetViewTargetwithBlend _returnvalue_2 _currentcamera 0.0 "VTBlend_Linear" 0.0 false)
        (Input|EnableInput _returnvalue_2)
        (Default|AddNewBaby _playerref)))
    (else
      (Development|PrintString "Not my baby")
      (Math|Integer|DecrementInt (Variables|/Game/ThirdPerson/Blueprints/BP_ThirdPersonCharacter.BP_ThirdPersonCharacter_C|GetbabyNumber _playerref)
        (:%20%20
          (Game|Player|SetViewTargetwithBlend _returnvalue _currentcamera 0.0 "VTBlend_Linear" 0.0 false)
          (Input|EnableInput _playerref _returnvalue)
          (Default|RemoveBaby _playerref)))))
  (bind _outactors (Actor|GetAllActorsOfClasswithTag "/Game/myFolder/BP_Baby.BP_Baby_C" "fish"))
  (for _array_element _outactors
    (Actor|DestroyActor _array_element))
  (Actor|DestroyActor))

(event Custom|Fish%20Baby)

(event EventBeginPlay)

(event Collision|EventActorBeginOverlap
  (params (OtherActor :type Actor%20Object%20Reference)))

(event EventTick
  (params (DeltaSeconds :type Float%20%28single-precision%29)))

(fn ConstructionScript)