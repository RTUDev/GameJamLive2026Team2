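; BP_Enemy is an enemy actor that shows a play-game prompt when the third-person character comes near it.
; PlayGameText is hidden at BeginPlay, shown when BP_ThirdPersonCharacter enters the Box trigger and hidden again when it leaves.
; Both overlap events set the character's CurrentEnemy to this actor, so leaving the trigger does not clear that reference.
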(event OnComponentBeginOverlap(Box)
  (params (OverlappedComponent :type Primitive%20Component%20Object%20Reference) (OtherActor :type Actor%20Object%20Reference) (OtherComp :type Primitive%20Component%20Object%20Reference) (OtherBodyIndex :type Integer) (bFromSweep :type Boolean) (SweepResult :type Hit%20Result%20Structure%20%28by%20ref%29))
  (bind _asbp_third_person_character (Utilities|Casting|CastToBP_ThirdPersonCharacter OtherActor))
  (Utilities|IsValid _asbp_third_person_character
    (:Is%20Valid
      (Rendering|SetVisibility (Variables|Default|GetplayGameText) true false)
      (Variables|/Game/ThirdPerson/Blueprints/BP_ThirdPersonCharacter.BP_ThirdPersonCharacter_C|SetcurrentEnemy _asbp_third_person_character self))))

(event OnComponentEndOverlap(Box)
  (params (OverlappedComponent :type Primitive%20Component%20Object%20Reference) (OtherActor :type Actor%20Object%20Reference) (OtherComp :type Primitive%20Component%20Object%20Reference) (OtherBodyIndex :type Integer))
  (bind _asbp_third_person_character (Utilities|Casting|CastToBP_ThirdPersonCharacter OtherActor))
  (Utilities|IsValid _asbp_third_person_character
    (:Is%20Valid
      (Rendering|SetVisibility (Variables|Default|GetplayGameText) false false)
      (Variables|/Game/ThirdPerson/Blueprints/BP_ThirdPersonCharacter.BP_ThirdPersonCharacter_C|SetcurrentEnemy _asbp_third_person_character self))))

(event EventBeginPlay
  (Rendering|SetVisibility (Variables|Default|GetplayGameText) false false))

(event Collision|EventActorBeginOverlap
  (params (OtherActor :type Actor%20Object%20Reference)))

(event EventTick
  (params (DeltaSeconds :type Float%20%28single-precision%29)))

(fn ConstructionScript)