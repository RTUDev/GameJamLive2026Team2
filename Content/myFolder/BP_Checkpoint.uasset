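; Checkpoint actor that teleports the third-person character to a linked checkpoint and switches the camera when it overlaps the box.
; With both neighbouring cameras valid, the character's LooksRight flag picks the side, offsetting the landing along Y and setting the view target and CurrentCamera.
; Without a left camera it always goes right; without a right camera or next checkpoint it does nothing.
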(event OnComponentBeginOverlap(Box)
  (params (OverlappedComponent :type Primitive%20Component%20Object%20Reference) (OtherActor :type Actor%20Object%20Reference) (OtherComp :type Primitive%20Component%20Object%20Reference) (OtherBodyIndex :type Integer) (bFromSweep :type Boolean) (SweepResult :type Hit%20Result%20Structure%20%28by%20ref%29))
  (bind _returnvalue (Game|GetPlayerController 0))
  (bind _nextcheckpoint (Variables|Default|GetNextCheckpoint))
  (bind _returnvalue_2 (Transformation|GetActorLocation _nextcheckpoint))
  (bind _asbp_third_person_character (Utilities|Casting|CastToBP_ThirdPersonCharacter OtherActor))
  (Utilities|IsValid _asbp_third_person_character
    (:Is%20Valid
      (Utilities|IsValid _nextcheckpoint
        (:Is%20Valid
          (Utilities|IsValid (Variables|/Game/myFolder/BP_Camera.BP_Camera_C|GetNextCameraRight (Variables|/Game/ThirdPerson/Blueprints/BP_ThirdPersonCharacter.BP_ThirdPersonCharacter_C|GetCurrentCamera _asbp_third_person_character))
            (:Is%20Valid
              (Utilities|IsValid (Variables|/Game/myFolder/BP_Camera.BP_Camera_C|GetNextCameraLeft (Variables|/Game/ThirdPerson/Blueprints/BP_ThirdPersonCharacter.BP_ThirdPersonCharacter_C|GetCurrentCamera _asbp_third_person_character))
                (:Is%20Valid
                  (if (Variables|/Game/ThirdPerson/Blueprints/BP_ThirdPersonCharacter.BP_ThirdPersonCharacter_C|GetlooksRight _asbp_third_person_character)
                    (Transformation|SetActorLocation _asbp_third_person_character (+ _returnvalue_2 "0.000000,100.000000,0.000000") false true :!label _label)
                    (Game|Player|SetViewTargetwithBlend _returnvalue (Variables|/Game/myFolder/BP_Camera.BP_Camera_C|GetNextCameraRight (Variables|/Game/ThirdPerson/Blueprints/BP_ThirdPersonCharacter.BP_ThirdPersonCharacter_C|GetCurrentCamera _asbp_third_person_character)) 0.0 "VTBlend_Linear" 0.0 false)
                    (Variables|/Game/ThirdPerson/Blueprints/BP_ThirdPersonCharacter.BP_ThirdPersonCharacter_C|SetCurrentCamera _asbp_third_person_character (Variables|/Game/myFolder/BP_Camera.BP_Camera_C|GetNextCameraRight (Variables|/Game/ThirdPerson/Blueprints/BP_ThirdPersonCharacter.BP_ThirdPersonCharacter_C|GetCurrentCamera _asbp_third_person_character)))
                    (else
                      (Transformation|SetActorLocation _asbp_third_person_character (+ _returnvalue_2 "0.000000,-100.000000,0.000000") false true)
                      (Game|Player|SetViewTargetwithBlend _returnvalue (Variables|/Game/myFolder/BP_Camera.BP_Camera_C|GetNextCameraLeft (Variables|/Game/ThirdPerson/Blueprints/BP_ThirdPersonCharacter.BP_ThirdPersonCharacter_C|GetCurrentCamera _asbp_third_person_character)) 0.0 "VTBlend_Linear" 0.0 false)
                      (Variables|/Game/ThirdPerson/Blueprints/BP_ThirdPersonCharacter.BP_ThirdPersonCharacter_C|SetCurrentCamera _asbp_third_person_character (Variables|/Game/myFolder/BP_Camera.BP_Camera_C|GetNextCameraLeft (Variables|/Game/ThirdPerson/Blueprints/BP_ThirdPersonCharacter.BP_ThirdPersonCharacter_C|GetCurrentCamera _asbp_third_person_character))))))
                (:Is%20Not%20Valid
                  (goto _label))))))))))

(event EventBeginPlay)

(event Collision|EventActorBeginOverlap
  (params (OtherActor :type Actor%20Object%20Reference)))

(event EventTick
  (params (DeltaSeconds :type Float%20%28single-precision%29)))

(fn ConstructionScript)