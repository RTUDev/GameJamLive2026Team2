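; BP_Cup is a clickable cup in a shell-game minigame, each hiding a baby.
; Timelines lower the cup to RandomCupSlot, then shuffle cup and baby there along RandomInt-chosen straight, front or behind paths before enabling clicks.
; Clicking locks all cups and reverses the float timeline to lift this one.
; A dance baby adds to the player's babies, otherwise one is removed; camera and input return, and cups and tagged babies are destroyed.
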(event EventBeginPlay)

(event Collision|EventActorBeginOverlap
  (params (OtherActor :type Actor%20Object%20Reference)))

(event EventTick
  (params (DeltaSeconds :type Float%20%28single-precision%29)))

(event MouseInput|EventActorOnClicked
  (params (ButtonPressed :type Key%20Structure :default "None"))
  (bind _returnvalue (Transformation|GetActorLocation))
  (bind _returnvalue_2 (Game|GetPlayerController 0))
  (bind _returnvalue_3 (Transformation|GetActorLocation))
  (bind _returnvalue_4 (Game|GetPlayerController 0))
  (bind _returnvalue_5 (Game|GetPlayerController 0))
  (bind _returnvalue_6 (Transformation|GetActorLocation))
  (bind _returnvalue_7 (Game|GetPlayerController 0))
  (bind _playerref (Variables|Default|GetplayerRef))
  (bind _randomcupslot (Variables|Default|GetrandomCupSlot))
  (bind _randomcupslot_2 (Variables|Default|GetrandomCupSlot))
  (bind _returnvalue_8 (Transformation|GetActorLocation _randomcupslot))
  (bind _returnvalue_9 (Transformation|GetActorLocation _randomcupslot))
  (bind _returnvalue_10 (Transformation|GetActorLocation _randomcupslot))
  (bind _currentcamera (Variables|/Game/ThirdPerson/Blueprints/BP_ThirdPersonCharacter.BP_ThirdPersonCharacter_C|GetCurrentCamera _playerref))
  (if (not (Variables|Default|GetwasClicked))
    (bind _outactors (Actor|GetAllActorsOfClass "BP_Cup_C"))
    (for _array_element _outactors
      (Variables|BP_Cup_C|SetwasClicked _array_element true))
    (bind _newtrack_0 (Timeline|FloatingDownTimeline Reverse)
      (:Update
        (if (Variables|Default|GetwasClicked)
          (Transformation|SetActorLocation (Math|Vector|Lerp(Vector) (Math|Vector|MakeVector (.x _returnvalue_3) (.y _returnvalue_3) (.z _returnvalue_3)) (Math|Vector|MakeVector (.x _returnvalue_3) (.y _returnvalue_3) (.z (Variables|Default|GetpositionUp))) (/ _newtrack_0 4e+01)) false false)
          (else
            (Utilities|IsValid _randomcupslot_2
              (:Is%20Valid
                (Transformation|SetActorLocation (Math|Vector|Lerp(Vector) (Math|Vector|MakeVector (.x _returnvalue_6) (.y _returnvalue_6) (.z _returnvalue_6)) (Math|Vector|MakeVector (.x _returnvalue_6) (.y _returnvalue_6) (.z (Transformation|GetActorLocation _randomcupslot_2))) (/ _newtrack_0 4e+01)) false false))))))
      (:Finished
        (if (not (Variables|Default|GetwasClicked))
          (bind (_direction _trackalpha _trackfront _trackbehind) (Timeline|ShuffleTimeline PlayFromStart)
            (:Update
              (switch int (Variables|Default|GetrandomInt)
                (:0
                  (Utilities|IsValid _randomcupslot
                    (:Is%20Valid
                      (Transformation|SetActorLocation (Math|Vector|Lerp(Vector) _returnvalue (Math|Vector|MakeVector (.x _returnvalue_9) (+ (.y _returnvalue_9) _trackfront) (.z _returnvalue_9)) _trackalpha) false false)
                      (Transformation|SetActorLocation (Variables|Default|GetmyBaby) (Math|Vector|Lerp(Vector) _returnvalue (Math|Vector|MakeVector (.x _returnvalue_9) (+ (.y _returnvalue_9) _trackfront) (.z _returnvalue_9)) _trackalpha) false false))))
                (:1
                  (Utilities|IsValid _randomcupslot
                    (:Is%20Valid
                      (Transformation|SetActorLocation (Math|Vector|Lerp(Vector) _returnvalue (Math|Vector|MakeVector (.x _returnvalue_10) (.y _returnvalue_10) (.z _returnvalue_10)) _trackalpha) false false)
                      (Transformation|SetActorLocation (Variables|Default|GetmyBaby) (Math|Vector|Lerp(Vector) _returnvalue (Math|Vector|MakeVector (.x _returnvalue_10) (.y _returnvalue_10) (.z _returnvalue_10)) _trackalpha) false false))))
                (:2
                  (Utilities|IsValid _randomcupslot
                    (:Is%20Valid
                      (Transformation|SetActorLocation (Math|Vector|Lerp(Vector) _returnvalue (Math|Vector|MakeVector (.x _returnvalue_8) (+ (.y _returnvalue_8) _trackbehind) (.z _returnvalue_8)) _trackalpha) false false)
                      (Transformation|SetActorLocation (Variables|Default|GetmyBaby) (Math|Vector|Lerp(Vector) _returnvalue (Math|Vector|MakeVector (.x _returnvalue_8) (+ (.y _returnvalue_8) _trackbehind) (.z _returnvalue_8)) _trackalpha) false false))))))
            (:Finished
              (Variables|/Script/Engine.PlayerController|SetbShowMouseCursor _returnvalue_7 true)
              (Variables|/Script/Engine.PlayerController|SetbEnableClickEvents _returnvalue_7 true)))
          (else
            (Utilities|IsValid _playerref
              (:Is%20Valid
                (bind _outactors_2 (Actor|GetAllActorsOfClass "BP_Cup_C"))
                (for _array_element_2 _outactors_2
                  _)
                (if (Variables|/Game/myFolder/BP_Baby.BP_Baby_C|GetisDanceBaby (Variables|Default|GetmyBaby))
                  (Math|Integer|IncrementInt (Variables|/Game/ThirdPerson/Blueprints/BP_ThirdPersonCharacter.BP_ThirdPersonCharacter_C|GetbabyNumber _playerref)
                    (:%20%20
                      (Game|Player|SetViewTargetwithBlend _returnvalue_4 _currentcamera 0.0 "VTBlend_Linear" 0.0 false)
                      (Input|EnableInput _playerref _returnvalue_4)
                      (Default|AddNewBaby _playerref)))
                  (else
                    (Math|Integer|DecrementInt (Variables|/Game/ThirdPerson/Blueprints/BP_ThirdPersonCharacter.BP_ThirdPersonCharacter_C|GetbabyNumber _playerref)
                      (:%20%20
                        (Game|Player|SetViewTargetwithBlend _returnvalue_5 _currentcamera 0.0 "VTBlend_Linear" 0.0 false)
                        (Input|EnableInput _playerref _returnvalue_5)
                        (Default|RemoveBaby _playerref)))))
                (Variables|/Script/Engine.PlayerController|SetbShowMouseCursor _returnvalue_2 false)
                (Variables|/Script/Engine.PlayerController|SetbEnableClickEvents _returnvalue_2 false)
                (bind _outactors_3 (Actor|GetAllActorsOfClasswithTag "/Game/myFolder/BP_Baby.BP_Baby_C" "cup"))
                (for _array_element_3 _outactors_3
                  (Actor|DestroyActor _array_element_3))
                (bind _outactors_4 (Actor|GetAllActorsOfClass "BP_Cup_C"))
                (for _array_element_4 _outactors_4
                  (Actor|DestroyActor _array_element_4))))))))))

(fn ConstructionScript
  (Variables|Default|SetpositionUp (Transformation|GetActorLocation)))